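; BP_Terrain is a terrain actor that links cursor hover to a hex grid and holds procedural mesh data.
; Each Tick it traces under the player's cursor and passes the hit's XY location to HexGrid.MouseOverGrid.
; CheckWorkflow stops its timer at the Create Triangles state and draws a capped number of debug vertex points.
; The looping timer setup and mesh section creation are disconnected, so neither runs.
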(event Custom|Event%20CheckWorkflow
  (switch Utilities|FlowControl|Switch|SwitchonEnum_TerrainWorkflowState (Variables|Default|GetWorkFlowState)
    (:CreateTriangles
      (Utilities|Time|ClearandInvalidateTimerbyHandle (Variables|Default|GetWorkflowCheckTimerHandle))
      (CallFunction|DrawDebugVertices 10000))))

(event EventTick
  (params (DeltaSeconds :type Float%20%28single-precision%29))
  (bind _returnvalue (Game|GetPlayerController 0))
  (bind (_hitresult _returnvalue_2) (Game|Player|GetHitResultUnderCursorbyChannel _returnvalue "TraceTypeQuery1" false))
  (bind _location (Collision|BreakHitResult _hitresult))
  (bind (_x _y) (Math|Vector|BreakVector _location))
  (bind _hexgrid (Variables|Default|GetHexGrid)
    (:then
      (if _returnvalue_2
        (Class|HexGrid|MouseOverGrid _hexgrid (Math|Vector2D|MakeVector2D _x _y))))
    (:else)))

(fn ConstructionScript)

(fn DrawDebugVertices
  (params (Limit :type Integer))
  (for (_array_element _array_index) (Variables|Default|GetVertices)
    (if (or (< _array_index Limit) (== Limit -1))
      (Rendering|Debug|DrawDebugPoint _array_element 5.0 "(R=0.000000,G=0.195179,B=1.000000,A=1.000000)" 1e+02)
      (else
        (return)))))