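; BP_HexGrid is a hex grid Blueprint whose visible logic consists mainly of debug helpers for its tile data.
; DrawDebugCenterPoint draws points at tile 2D positions, and ShowDebugIndices prints each tile's index looked up by axial coordinate in TileIndices.
; CheckWorkflow switches on WorkFlowState without acting.
; BeginPlay is empty, and the looping timer meant to poll CheckWorkflow is disconnected, along with the parent BeginPlay call.
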(event Custom|CheckWorkflow
  (switch Utilities|FlowControl|Switch|SwitchonEnum_HexGridWorkflowState (Variables|Default|GetWorkFlowState)))

(event EventBeginPlay)

(fn ConstructionScript)

(fn DrawDebugCenterPoint
  (params (Number :type Integer))
  (for _index (range 0 Number)
    (Rendering|Debug|DrawDebugPoint (Math|Vector|MakeVector (.X (Math|Vector2D|BreakVector2D (.Position2D (Utilities|Struct|BreakStructHexTileData (Utilities|Array|Get(acopy) (Variables|Default|GetTiles) _index))))) (.Y (Math|Vector2D|BreakVector2D (.Position2D (Utilities|Struct|BreakStructHexTileData (Utilities|Array|Get(acopy) (Variables|Default|GetTiles) _index))))) 0.0) 5.0 "(R=0.000000,G=0.084431,B=1.000000,A=1.000000)" 1e+02)))

(fn ShowDebugIndices
  (params (Number :type Integer))
  (for _index (range 0 Number)
    (if (.ReturnValue (Utilities|Map|Find (Variables|Default|GetTileIndices) (.AxialCoord (Utilities|Struct|BreakStructHexTileData (Utilities|Array|Get(acopy) (Variables|Default|GetTiles) _index)))))
      (Development|PrintString (Utilities|String|ToString(Integer) (.Value (Utilities|Map|Find (Variables|Default|GetTileIndices) (.AxialCoord (Utilities|Struct|BreakStructHexTileData (Utilities|Array|Get(acopy) (Variables|Default|GetTiles) _index)))))) true true "(R=0.000000,G=0.660000,B=1.000000,A=1.000000)" 1e+01)
      (else
        (Development|PrintString "Error!!!" true true "(R=0.000000,G=0.660000,B=1.000000,A=1.000000)" 1e+01)))))