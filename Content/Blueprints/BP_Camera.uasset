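; BP_Camera is a top-down terrain camera pawn that pans, rotates and zooms over a BP_Terrain.
; Enhanced Input drives spring-arm zoom, plus drag-move and pitch-limited rotation gated by the terrain's left and right hold states.
; A looping timer checks screen edges for cursor scrolling.
; Pans follow camera yaw, scale with zoom and clamp to bounds from the terrain size, which another timer polls for at startup.
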(event Custom|SetTerrain
  (bind _boundaryscalar (Variables|Default|GetBoundaryScalar))
  (bind _boundaryscalar_2 (Variables|Default|GetBoundaryScalar))
  (bind _returnvalue (* _boundaryscalar_2 -1.0))
  (bind _outactors (Actor|GetAllActorsOfClass "/Game/Blueprints/BP_Terrain.BP_Terrain_C"))
  (if (== (Utilities|Array|Length _outactors) 1)
    (Variables|Default|SetTerrain (Utilities|Array|Get(acopy) _outactors))
    (Variables|Default|SetLocMin (Math|Vector|MakeVector (* (Variables|/Script/MapTestCPP.Terrain|GetTerrainWidth (Variables|Default|GetTerrain)) _returnvalue) (* _returnvalue (Variables|/Script/MapTestCPP.Terrain|GetTerrainHeight (Variables|Default|GetTerrain))) -1e+02))
    (Variables|Default|SetLocMax (Math|Vector|MakeVector (* (Variables|/Script/MapTestCPP.Terrain|GetTerrainWidth (Variables|Default|GetTerrain)) _boundaryscalar) (* _boundaryscalar (Variables|/Script/MapTestCPP.Terrain|GetTerrainHeight (Variables|Default|GetTerrain))) 1e+02))
    (Utilities|Time|ClearandInvalidateTimerbyHandle (Variables|Default|GetSetTerrainTimerHandler))))

(event Custom|Scroll%20Screen
  (CallFunction|Scroll))

(event Input|EnhancedActionEvents|EnhancedInputActionIA_CameraRotate
  (params (ActionValue :type Vector%202D%20Structure) (ElapsedSeconds :type Float%20%28double-precision%29) (TriggeredSeconds :type Float%20%28double-precision%29) (InputAction :type Input%20Action%20Object%20Reference :default "/Game/Input/Actions/Camera/IA_CameraRotate.IA_CameraRotate"))
  (bind (_x _y) (Math|Vector2D|BreakVector2D ActionValue))
  (Utilities|IsValid (Variables|Default|GetTerrain)
    (:Is%20Valid
      (bind _returnvalue (Class|Terrain|IsRightHold (Variables|Default|GetTerrain)))
      (if _returnvalue
        (Utilities|FlowControl|Sequence
          (:then_0
            (Pawn|Input|AddControllerYawInput _x))
          (:then_1
            (Pawn|Input|AddControllerPitchInput (* _y -1.0))))))))

(event Input|EnhancedActionEvents|EnhancedInputActionIA_CameraZoomOut
  (params (ActionValue :type Boolean) (ElapsedSeconds :type Float%20%28double-precision%29) (TriggeredSeconds :type Float%20%28double-precision%29) (InputAction :type Input%20Action%20Object%20Reference :default "/Game/Input/Actions/Camera/IA_CameraZoomOut.IA_CameraZoomOut"))
  (Variables|/Script/Engine.SpringArmComponent|SetTargetArmLength (Variables|Default|GetSpringArm) (Math|Float|Clamp(Float) (+ (Variables|/Script/Engine.SpringArmComponent|GetTargetArmLength (Variables|Default|GetSpringArm)) 4e+03) 1e+04 1e+05)))

(event Input|EnhancedActionEvents|EnhancedInputActionIA_CameraZoomIn
  (params (ActionValue :type Boolean) (ElapsedSeconds :type Float%20%28double-precision%29) (TriggeredSeconds :type Float%20%28double-precision%29) (InputAction :type Input%20Action%20Object%20Reference :default "/Game/Input/Actions/Camera/IA_CameraZoomIn.IA_CameraZoomIn"))
  (Variables|/Script/Engine.SpringArmComponent|SetTargetArmLength (Variables|Default|GetSpringArm) (Math|Float|Clamp(Float) (- (Variables|/Script/Engine.SpringArmComponent|GetTargetArmLength (Variables|Default|GetSpringArm)) 4e+03) 1e+04 1e+05)))

(event Input|EnhancedActionEvents|EnhancedInputActionIA_CameraMove
  (params (ActionValue :type Vector%202D%20Structure) (ElapsedSeconds :type Float%20%28double-precision%29) (TriggeredSeconds :type Float%20%28double-precision%29) (InputAction :type Input%20Action%20Object%20Reference :default "/Game/Input/Actions/Camera/IA_CameraMove.IA_CameraMove"))
  (Utilities|IsValid (Variables|Default|GetTerrain)
    (:Is%20Valid
      (bind _returnvalue (Class|Terrain|IsLeftHold (Variables|Default|GetTerrain)))
      (if _returnvalue
        (CallFunction|Move ActionValue)))))

(event EventBeginPlay
  (bind _returnvalue (Game|GetPlayerController 0))
  (bind _playercameramanager (Variables|/Script/Engine.PlayerController|GetPlayerCameraManager _returnvalue))
  (Game|Player|SetViewTargetwithBlend (Game|GetPlayerController 0) self 0.0 "VTBlend_Linear" 0.0 false)
  (Input|AddMappingContext (PlayerController|LocalPlayerSubsystems|GetEnhancedInputLocalPlayerSubsystem (Game|GetPlayerController 0)) "/Game/Input/IMC_TerrainCamera.IMC_TerrainCamera" 0 "(bIgnoreAllPressedKeysUntilRelease=True,bForceImmediately=False,bNotifyUserSettings=False)")
  (bind _returnvalue_2 (Utilities|Time|SetTimerbyEvent (delegate Custom|SetTerrain) 1.0 true))
  (Variables|Default|SetSetTerrainTimerHandler _returnvalue_2)
  (Variables|/Script/Engine.SpringArmComponent|SetbUsePawnControlRotation (Variables|Default|GetSpringArm) true)
  (Pawn|Input|AddControllerPitchInput 16.0)
  (Variables|/Script/Engine.SpringArmComponent|SetTargetArmLength (Variables|Default|GetSpringArm) 3e+04)
  (Variables|/Script/Engine.PlayerCameraManager|SetViewPitchMax _playercameramanager -1e+01)
  (Variables|/Script/Engine.PlayerCameraManager|SetViewPitchMin _playercameramanager -7e+01)
  (Utilities|Time|SetTimerbyEvent (delegate Custom|Scroll%20Screen) 0.03 true))

(event EventTick
  (params (DeltaSeconds :type Float%20%28single-precision%29)))

(fn ConstructionScript)

(fn ScrollLeft
  (bind _returnvalue (Viewport|GetViewportSize))
  (bind _returnvalue_2 (Class|WidgetLayoutLibrary|GetMousePositiononViewport))
  (if (> (- 1.0 (Math|Float|Clamp(Float) (Math|Float|NormalizetoRange (* (Class|WidgetLayoutLibrary|GetViewportScale) (.x _returnvalue_2)) 0.0 (* (.x (Viewport|GetViewportSize)) 0.005)))) 0.0)
    (CallFunction|OffsetbyVector (Math|Vector|MakeVector 0.0 (* (/ (.x _returnvalue) (.y _returnvalue)) -0.7) 0.0) (Variables|Default|GetScrollScalar))))

(fn ScrollRight
  (bind _returnvalue (Viewport|GetViewportSize))
  (bind _returnvalue_2 (Viewport|GetViewportSize))
  (bind _returnvalue_3 (Class|WidgetLayoutLibrary|GetMousePositiononViewport))
  (if (> (Math|Float|Clamp(Float) (Math|Float|NormalizetoRange (* (Class|WidgetLayoutLibrary|GetViewportScale) (.x _returnvalue_3)) (* (.x _returnvalue_2) 0.995) (.x _returnvalue_2))) 0.0)
    (CallFunction|OffsetbyVector (Math|Vector|MakeVector 0.0 (* (/ (.x _returnvalue) (.y _returnvalue)) 0.7) 0.0) (Variables|Default|GetScrollScalar))))

(fn ScrollUp
  (bind _returnvalue (Class|WidgetLayoutLibrary|GetMousePositiononViewport))
  (if (> (- 1.0 (Math|Float|Clamp(Float) (Math|Float|NormalizetoRange (* (Class|WidgetLayoutLibrary|GetViewportScale) (.y _returnvalue)) 0.0 (* (.y (Viewport|GetViewportSize)) 0.005)))) 0.0)
    (CallFunction|OffsetbyVector (Math|Vector|MakeVector 1.0 0.0 0.0) (Variables|Default|GetScrollScalar))))

(fn ScrollDown
  (bind _returnvalue (Viewport|GetViewportSize))
  (bind _returnvalue_2 (Class|WidgetLayoutLibrary|GetMousePositiononViewport))
  (if (> (Math|Float|Clamp(Float) (Math|Float|NormalizetoRange (* (Class|WidgetLayoutLibrary|GetViewportScale) (.y _returnvalue_2)) (* (.y _returnvalue) 0.99) (.y _returnvalue))) 0.0)
    (CallFunction|OffsetbyVector (Math|Vector|MakeVector -1.0 0.0 0.0) (Variables|Default|GetScrollScalar))))

(fn Move
  (params (ActionValue :type Vector%202D%20Structure))
  (bind (_x _y) (Math|Vector2D|BreakVector2D ActionValue))
  (CallFunction|OffsetbyVector (Math|Vector|MakeVector _y _x 0.0) (Variables|Default|GetMoveScalar)))

(fn Scroll
  (CallFunction|ScrollLeft)
  (CallFunction|ScrollRight)
  (CallFunction|ScrollUp)
  (CallFunction|ScrollDown))

(fn OffsetbyVector
  (params (Offset :type Vector) (Scalar :type Float%20%28double-precision%29))
  (bind _self self)
  (Transformation|AddActorLocalOffset _self (Math|Vector|RotateVector (* (* (/ (Variables|/Script/Engine.SpringArmComponent|GetTargetArmLength (Variables|Default|GetSpringArm)) 1e+02) Scalar) Offset) (Math|Rotator|MakeRotator 0.0 0.0 (.Yaw (Math|Rotator|BreakRotator (Transformation|GetWorldRotation (Variables|Default|GetCamera)))))) false false)
  (Transformation|SetActorLocation _self (Class|KismetMathLibrary|VectorBoundedtoBox (Transformation|GetActorLocation _self) (Variables|Default|GetLocMin) (Variables|Default|GetLocMax)) false false))